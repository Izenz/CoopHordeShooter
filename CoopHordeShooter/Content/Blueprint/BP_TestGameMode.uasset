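; Test game mode that handles enemy spawning and awards score for kills.
; SpawnNewEnemy runs an EQS query for spawn locations, then randomly spawns an advanced AI or, more often, a tracker ball at each result.
; On BeginPlay it binds to OnActorKilled, adding score to the killer's HSPlayerState for non-player pawn victims and refreshing that player pawn's score widget.
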(event `self.SpawnNewEnemy`
  (bind _returnvalue (`EnvQueryManager.RunEQSQuery` "/Game/Blueprint/EQS_FindSpawnLocation.EQS_FindSpawnLocation" self "RandomBest25Pct"))
  (add `EnvQueryInstanceBlueprintWrapper.OnQueryFinishedEvent` _returnvalue (delegate `OnQueryFinishedEvent_Event_0`)))

(event `OnQueryFinishedEvent_Event_0`
  (params (QueryInstance :type "EnvQueryInstanceBlueprintWrapper Object Reference") (QueryStatus :type "EEnvQueryStatus Enum" :default "Processing"))
  (switch `EEnvQueryStatus` QueryStatus
    (:`Success`
      (for _array_element (`EnvQueryInstanceBlueprintWrapper.GetResultsAsLocations` QueryInstance)
        (`|SpawnActorFromClass` (select `bool` (<= (`KismetMathLibrary.RandomFloatInRange` 0.0 100.0) 30.0) :`false` "/Game/Blueprint/BP_TrackerBall.BP_TrackerBall_C" :`true` "/Game/Blueprint/BP_Advanced_AI.BP_Advanced_AI_C" :!type "Actor Class Reference") (`KismetMathLibrary.MakeTransform` _array_element) "AdjustIfPossibleButDontSpawnIfColliding" "OverrideRootScale" null null)))))

(event `self.ReceiveBeginPlay`
  (add `self.OnActorKilled` (delegate `OnActorKilled_Event_0`)))

(event `OnActorKilled_Event_0` :!signature `self.OnActorKilled`
  (params (VictimActor :type "Actor Object Reference") (KillerActor :type "Actor Object Reference") (KillerController :type "Controller Object Reference"))
  (bind _returnvalue (`Controller.K2_GetPawn` KillerController))
  (`/Engine/EditorBlueprintResources/StandardMacros.IsValid` KillerController
    (:`Is Valid`
      ;[1 1 1] Do not reward for killing other players
      (bind _aspawn (cast `Pawn` VictimActor))
      (if (not (`Pawn.IsPlayerControlled` _aspawn))
        (bind _ashsplayer_state (cast `HSPlayerState` (`Pawn.PlayerState` _returnvalue)))
        (`HSPlayerState.AddScore` _ashsplayer_state 20.0)
        (bind _asbp_player_pawn (cast `/Game/Blueprint/BP_PlayerPawn` _returnvalue))
        (`/Game/UI/WBP_Score.UpdateScore` (`/Game/Blueprint/BP_PlayerPawn.ScoreWidget` _asbp_player_pawn) (`PlayerState.Score` _ashsplayer_state))))))

(fn `UserConstructionScript`)