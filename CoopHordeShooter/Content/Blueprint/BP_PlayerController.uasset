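; Player controller that manages the player's HUD: score, health indicators and the death screen.
; On BeginPlay the local controller creates the score widget, which UpdatePlayerScore later refreshes.
; A lazily created indicator widget binds to health components and releases them through ClientRPC when OnPlayerKilled fires.
; DrawDeathScreen shows the death widget locally, switching to UI-only input with a visible cursor.
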(event `ClientRPC`
  (params (HealthComp :type "HSHealthComponent Object Reference"))
  (`/Game/UI/WBP_HealthIndicator.ReleaseIndicator` (`self.HealthIndicatorWidget`) HealthComp))

(event `self.OnPlayerKilled`
  (params (HealthComp :type "HSHealthComponent Object Reference"))
  (`self.ClientRPC` HealthComp))

(event `self.ReceiveBeginPlay`
  (if (`self.IsLocalController`)
    (bind _returnvalue (`|CreateWidget` "/Game/UI/WBP_Score.WBP_Score_C"))
    (bind _output_get (set `self.ScoreWidget` _returnvalue))
    (`UserWidget.AddToViewport` _output_get 0)))

(event `BindIndicatorToHealth`
  (params (`Health Comp` :type "HSHealthComponent Object Reference"))
  (bind _healthindicatorwidget (`self.HealthIndicatorWidget`))
  (`/Engine/EditorBlueprintResources/StandardMacros.IsValid` _healthindicatorwidget
    (:`Is Valid`
      _)
    (:`Is Not Valid`
      (bind _returnvalue (`|CreateWidget` "/Game/UI/WBP_HealthIndicator.WBP_HealthIndicator_C"))
      (bind _output_get (set `self.HealthIndicatorWidget` _returnvalue))
      (`UserWidget.AddToViewport` _output_get 0)))
  (`/Game/UI/WBP_HealthIndicator.BindIndicatorToHealthComp` _healthindicatorwidget `Health Comp`))

(event `self.UpdatePlayerScore`
  (params (NewScore :type "Float (single-precision)"))
  (bind _scorewidget (`self.ScoreWidget`))
  (`/Engine/EditorBlueprintResources/StandardMacros.IsValid` _scorewidget
    (:`Is Valid`
      (`/Game/UI/WBP_Score.UpdateScore` _scorewidget NewScore))))

(event `self.DrawDeathScreen`
  (if (`self.IsLocalController`)
    (bind _returnvalue (`|CreateWidget` "/Game/UI/WBP_DeathScreen.WBP_DeathScreen_C"))
    (`UserWidget.AddToViewport` _returnvalue 0)
    (`WidgetBlueprintLibrary.SetInputMode_UIOnlyEx` self)
    (set `self.bShowMouseCursor` true)))

(fn `OnRep_HealthIndicatorWidget`)

(fn `UserConstructionScript`)